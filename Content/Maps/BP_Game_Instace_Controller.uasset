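; Game instance controller that handles level progression, restarts and returning to the main menu.
; LoadNextLevel steps LevelIndex through the Levels array, wraps to the first entry at the end, and opens that level by name.
; LoadMainMenu opens the first entry and resets the index, while RestartLevel reopens the current level.
; Next-level and restart calls also zero BotCount on Game_Mode_Controller after requesting the level open.
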(fn LoadNextLevel
  (bind _levels (Variables|Default|GetLevels))
  (bind _result (Math|Integer|IncrementInt (Variables|Default|GetLevel%20Index))
    (:%20%20
      (if (== _result (Utilities|Array|Length (Variables|Default|GetLevels)))
        (bind _output_get (Variables|Default|SetLevel%20Index 0))
        (Game|OpenLevel(byName) (Utilities|String|StringToName (Utilities|Array|Get(acopy) _levels _output_get)))
        (else
          (Game|OpenLevel(byName) (Utilities|String|StringToName (Utilities|Array|Get(acopy) _levels (Variables|Default|GetLevel%20Index))))))
      ;[1 1 1] Reset Bot Count
      (bind _asgame_mode_controller (Utilities|Casting|CastToGame_Mode_Controller (Game|GetGameMode)))
      (Variables|/Game/Maps/Game_Mode_Controller.Game_Mode_Controller_C|SetBot%20Count _asgame_mode_controller 0))))

(fn LoadMainMenu
  (Game|OpenLevel(byName) (Utilities|String|StringToName (Utilities|Array|Get(acopy) (Variables|Default|GetLevels))))
  (Variables|Default|SetLevel%20Index 0))

(fn RestartLevel
  (bind _returnvalue (Game|GetCurrentLevelName true))
  (Game|OpenLevel(byName) (Utilities|String|StringToName _returnvalue))
  (bind _asgame_mode_controller (Utilities|Casting|CastToGame_Mode_Controller (Game|GetGameMode)))
  (Variables|/Game/Maps/Game_Mode_Controller.Game_Mode_Controller_C|SetBot%20Count _asgame_mode_controller 0))