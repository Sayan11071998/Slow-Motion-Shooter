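; BP_MainMenu_Bot is a bot actor for the main menu that spawns a gun and opens the menu UI.
; On BeginPlay it attaches BP_Gun_Bot to the mesh's gun socket, adds WBP_MainMenu_UI and switches to UI-only input with the cursor shown.
; CheckForPlayer, not called in these graphs, line-traces from the head socket to the player's camera to set or clear the target based on sight, range and a lock timer.
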(event EventBeginPlay
  (bind _returnvalue (Game|GetPlayerController 0))
  (bind _skeletalmesh (Variables|Default|GetSkeletalMesh))
  ;[1 1 1] Spawn Gun
  (bind _returnvalue_2 (Game|SpawnActorfromClass "/Game/Blueprints/Weapons_Blueprints/BP_Gun_Bot.BP_Gun_Bot_C" (Transformation|GetSocketTransform _skeletalmesh "b_Gun" "RTS_World") "Undefined" 0 0))
  (bind _output_get (Variables|Default|SetGun _returnvalue_2))
  (Transformation|AttachComponentToComponent _output_get _skeletalmesh "b_Gun" "KeepWorld" "KeepWorld" "KeepWorld" true)
  (bind _returnvalue_3 (UserInterface|CreateWidget "/Game/Blueprints/Widget_Blueprints/WBP_MainMenu_UI.WBP_MainMenu_UI_C"))
  (UserInterface|Viewport|AddtoViewport _returnvalue_3 0)
  (Input|SetInputModeUIOnly _returnvalue _returnvalue_3 "DoNotLock" false)
  (Variables|/Script/Engine.PlayerController|SetbShowMouseCursor _returnvalue true))

(fn ConstructionScript)

(fn CheckforPlayer
  (bind _returnvalue (Game|GetPlayerCharacter 0))
  (bind _asbp_player_character (Utilities|Casting|CastToBP_Player_Character _returnvalue))
  (bind _outhit (Collision|LineTraceByChannel (.Location (Math|Transform|BreakTransform (Transformation|GetSocketTransform (Variables|Default|GetSkeletalMesh) "headSocket" "RTS_World"))) (+ (Transformation|GetActorLocation _returnvalue) (Variables|/Script/Engine.SceneComponent|GetRelativeLocation (Variables|/Game/Blueprints/Character_Blueprints/BP_Player_Character.BP_Player_Character_C|GetFirst%20Person%20Camera _asbp_player_character))) "TraceTypeQuery2" false 0 "None"))
  (if (!= (.HitActor (Collision|BreakHitResult _outhit)) 0)
    (if (== _returnvalue (.HitActor (Collision|BreakHitResult _outhit)))
      (if (< (Transformation|GetDistanceTo (.HitActor (Collision|BreakHitResult _outhit))) (Variables|Default|GetRange))
        (Variables|Default|SetDesiredRotation (Math|Rotator|FindLookatRotation (Transformation|GetActorLocation) (Transformation|GetActorLocation (.HitActor (Collision|BreakHitResult _outhit)))))
        (Variables|Default|SetTargetActor (.HitActor (Collision|BreakHitResult _outhit)))
        (else
          (if (not (Variables|Default|GetLockTimer)) :!label _label
            (Variables|Default|SetTargetActor 0))))
      (else
        (goto _label)))))