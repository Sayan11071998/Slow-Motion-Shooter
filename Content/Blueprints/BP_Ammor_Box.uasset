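; BP_Ammor_Box is an ammo pickup box that gradually refills the player's ammo while BP_Player_Character overlaps it.
; Tick runs a timer during overlap, moving one round per threshold interval if the player is below max, updating a text counter and playing audio.
; When the box empties, a timeline shrinks it from its starting scale to zero and then destroys it.
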(event Custom|On%20Destroy
  ;[1 1 1] Shrink & Destroy Cube
  (bind _alpha (Timeline|BoxShrink_Template Play)
    (:Update
      (Transformation|SetActorScale3D (Math|Vector|Lerp(Vector) (Variables|Default|GetCurrentScale) "0, 0, 0" _alpha)))
    (:Finished
      (Actor|DestroyActor))))

(event EventBeginPlay
  ;[1 1 1] Display Initial Ammo
  (Rendering|Components|TextRender|SetText (Variables|Default|GetTextRender) (Utilities|Text|ToText(Integer) (Variables|Default|GetAmmo%20Left)))
  ;[1 1 1] Get Current Scale
  (Variables|Default|SetCurrentScale (Transformation|GetActorScale3D)))

(event Collision|EventActorBeginOverlap
  (params (OtherActor :type Actor%20Object%20Reference))
  ;[1 1 1] Set Can Fill Ammo = true
  (bind _asbp_player_character (Utilities|Casting|CastToBP_Player_Character OtherActor))
  (Variables|Default|SetPlayer_REF _asbp_player_character)
  (Variables|Default|SetCanFillAmmo true))

(event EventTick
  (params (DeltaSeconds :type Float%20%28single-precision%29))
  (bind _player_ref (Variables|Default|GetPlayer_REF))
  ;[1 1 1] Fill Ammo
  (if (Variables|Default|GetCanFillAmmo)
    (bind _output_get (Variables|Default|SetFill%20Ammo%20Timer (+ (Variables|Default|GetFill%20Ammo%20Timer) DeltaSeconds)))
    (if (>= _output_get (Variables|Default|GetFill%20Ammo%20Threshold))
      (if (< (Variables|/Game/Blueprints/Character_Blueprints/BP_Player_Character.BP_Player_Character_C|GetCurrentAmmo _player_ref) (Variables|/Game/Blueprints/Character_Blueprints/BP_Player_Character.BP_Player_Character_C|GetMaxAmmo _player_ref))
        (Math|Integer|IncrementInt (Variables|/Game/Blueprints/Character_Blueprints/BP_Player_Character.BP_Player_Character_C|GetCurrentAmmo (Variables|Default|GetPlayer_REF))
          (:%20%20
            (bind _result (Math|Integer|DecrementInt (Variables|Default|GetAmmo%20Left))
              (:%20%20
                (Rendering|Components|TextRender|SetText (Variables|Default|GetTextRender) (Utilities|Text|ToText(Integer) _result))
                (Variables|Default|SetFill%20Ammo%20Timer 0.0)
                (Audio|Components|Audio|Play (Variables|Default|GetAudio) 0.0)
                (if (== (Variables|Default|GetAmmo%20Left) 0)
                  (if (Variables|Default|GetCanDestroy)
                    (Variables|Default|SetCanDestroy false)
                    (CallFunction|OnDestroy)))))))))))

(event Collision|EventActorEndOverlap
  (params (OtherActor :type Actor%20Object%20Reference))
  ;[1 1 1] Set Can Fill Ammo = false
  (Utilities|Casting|CastToBP_Player_Character OtherActor)
  (Variables|Default|SetCanFillAmmo false)
  (Variables|Default|SetFill%20Ammo%20Timer 0.0))

(fn ConstructionScript)